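; BP_Door_Actual is a door that swings open and closed by yawing its Rotator component.
; ActivateDoor clears IsClosed and plays DoorTL, whose track sets the Rotator's relative yaw, while DeactivateDoor sets IsClosed and reverses the same timeline.
; A separate Timeline also plays on BeginPlay and drives the same yaw.
; The construction script only calls its parent.
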(event `self.ReceiveBeginPlay`
  (bind (_direction _newtrack_0) (`Timeline|Timeline`)
    (:`Update`
      (`SceneComponent.K2_SetRelativeRotation` (`self.Rotator`) (`KismetMathLibrary.MakeRotator` 0.0 0.0 _newtrack_0) false false))))

(event `Activate Door`
  (set `self.isClosed` false)
  (bind (_direction _newtrack_0) (`Timeline|DoorTL` :!label _label)
    (:`Update`
      (`SceneComponent.K2_SetRelativeRotation` (`self.Rotator`) (`KismetMathLibrary.MakeRotator` 0.0 0.0 _newtrack_0) false false))))

(event `Deactivate Door`
  (set `self.isClosed` true)
  (goto _label :!via `Reverse`))

(fn `UserConstructionScript`
  (`parent.UserConstructionScript`))