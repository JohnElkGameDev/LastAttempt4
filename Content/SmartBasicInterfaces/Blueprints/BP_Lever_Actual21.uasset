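; Lever actor that the first-person player toggles with F while inside its Box trigger to activate or deactivate a referenced door.
; Box overlaps set PlayerInRange, and the actor enables its own input on BeginPlay to receive the key.
; Each press flips IsActive, calls ActivateDoor (when it was true) or DeactivateDoor on DoorReference, and plays or reverses a timeline that pitches LeverMovable.
; Debug prints remain.
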(event `Key|F`
  (params (Key :type "Key Structure"))
  (:`Pressed`
    (if (`self.playerInRange`)
      (`KismetSystemLibrary.PrintString` "is in range")
      (if (`self.isActive`)
        (`KismetSystemLibrary.PrintString` "is active")
        (set `self.isActive` false)
        (`/Game/SmartBasicInterfaces/Blueprints/BP_Door_Actual.Activate Door` (`self.doorReference`))
        (bind (_direction _newtrack_0) (`Timeline|TimelineAction` :!label _label)
          (:`Update`
            (`SceneComponent.K2_SetRelativeRotation` (`self.Lever_Movable`) (`KismetMathLibrary.MakeRotator` 0.0 _newtrack_0) false false)))
        (else
          (set `self.isActive` true)
          (`/Game/SmartBasicInterfaces/Blueprints/BP_Door_Actual.Deactivate Door` (`self.doorReference`))
          (goto _label :!via `Reverse`))))))

(event `self.Box.OnComponentBeginOverlap`
  (params (OverlappedComponent :type "PrimitiveComponent Object Reference") (OtherActor :type "Actor Object Reference") (OtherComp :type "PrimitiveComponent Object Reference") (OtherBodyIndex :type Integer) (bFromSweep :type Boolean) (SweepResult :type "HitResult Structure (by ref)"))
  (cast `/Game/FirstPerson/Blueprints/BP_FirstPersonCharacter` OtherActor)
  (set `self.playerInRange` true))

(event `self.Box.OnComponentEndOverlap`
  (params (OverlappedComponent :type "PrimitiveComponent Object Reference") (OtherActor :type "Actor Object Reference") (OtherComp :type "PrimitiveComponent Object Reference") (OtherBodyIndex :type Integer))
  (cast `/Game/FirstPerson/Blueprints/BP_FirstPersonCharacter` OtherActor)
  (set `self.playerInRange` false))

(event `self.ReceiveBeginPlay`
  (`self.EnableInput` (`GameplayStatics.GetPlayerController` 0)))

(fn `UserConstructionScript`
  (`parent.UserConstructionScript`))