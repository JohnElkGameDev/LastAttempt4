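; BP_LightsEnemy is a lighting actor that switches three spotlights according to the movement state of an enemy.
; Every Tick it reads IsMoving from the Enemy1 reference and sets the visibility of SpotLight, SpotLight1 and SpotLight2.
; The lights are hidden while the enemy moves and shown while it is not moving.
; It polls the flag each frame, with no event binding or change check.
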(event `self.ReceiveTick`
  (params (DeltaSeconds :type "Float (single-precision)"))
  (if (`/Game/Enemy/BP_Enemy.isMoving` (`self.Enemy1`))
    (`SceneComponent.SetVisibility` (`self.SpotLight2`) false false)
    (`SceneComponent.SetVisibility` (`self.SpotLight1`) false false)
    (`SceneComponent.SetVisibility` (`self.SpotLight`) false false)
    (else
      (`SceneComponent.SetVisibility` (`self.SpotLight2`) true false)
      (`SceneComponent.SetVisibility` (`self.SpotLight1`) true false)
      (`SceneComponent.SetVisibility` (`self.SpotLight`) true false))))

(fn `UserConstructionScript`)