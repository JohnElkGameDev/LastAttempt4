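; BP_Enemy is an enemy that teleports along a looping list of position points toward an attack on the player.
; A repeating timer advances it one point and randomly sets an IsMoving flag, cleared shortly after, which does not gate the move.
; After the last point, if MyDoor is open, it teleports in front of the player, changes game state and HUD, and pauses the game.
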(event `self.ReceiveBeginPlay`
  (`KismetSystemLibrary.K2_SetTimer` null "Move" (`self.MoveInterval`) true))

(event `Move`
  (if true
    (set `self.isMoving` (< (`KismetMathLibrary.RandomFloatInRange` 0.0 1.0) 0.2))
    (`self.K2_SetActorLocation` (`self.K2_GetActorLocation` (`|GetArrayItem` (`self.PosPoints`) (`self.CurrentPos`))))
    (set `self.CurrentPos` (mod (+ (`self.CurrentPos`) 1) (`KismetArrayLibrary.Array_Length` (`self.PosPoints`))))
    (`KismetSystemLibrary.K2_SetTimer` null "Moving" 1.0)
    (if (== (`self.CurrentPos`) 0)
      (if (not (`/Game/SmartBasicInterfaces/Blueprints/BP_Door_Actual.isClosed` (`self.myDoor`)))
        (`self.SpawnInFront`)))))

(event `Moving`
  (set `self.isMoving` false))

(event `SpawnInFront`
  (bind _returnvalue (`GameplayStatics.GetPlayerCharacter` 0))
  (`self.K2_SetActorLocation` (+ (* (`self.GetActorForwardVector` _returnvalue) (`self.SpawnDistance`)) (`self.K2_GetActorLocation` _returnvalue)))
  (bind _asbp_game_instance (cast `/Game/GameStates/BP_GameInstance` (`GameplayStatics.GetGameInstance`)))
  (`/Game/GameStates/BP_GameInstance.SetGameState` _asbp_game_instance "NewEnumerator3")
  (`/Game/HUD/WBP_HUD.UpdateHUD` (`self.HUDWidget`) "NewEnumerator3")
  (`GameplayStatics.SetGamePaused` true)
  (`WidgetBlueprintLibrary.SetInputMode_GameAndUIEx` (`GameplayStatics.GetPlayerController` 0) null))

(fn `UserConstructionScript`)