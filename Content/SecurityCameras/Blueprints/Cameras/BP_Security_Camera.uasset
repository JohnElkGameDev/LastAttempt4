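; Security camera actor that can feed a render target and be toggled between broken and fixed.
; BeginPlay adds a SceneCapture2D at the CameraScreen transform without a target, disabling every-frame capture after a brief delay.
; Updatecamera assigns the capture's render target.
; Break/Fix flip-flops between looping electric sparks and sound at random intervals while IsBroken, and playing a fix sound before clearing it.
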(event `self.ReceiveBeginPlay`
  (bind _returnvalue (`AddComponent|NODE_AddSceneCaptureComponent2D-0` :`RelativeTransform` (`SceneComponent.GetRelativeTransform` (`self.CameraScreen`))))
  (set `SceneCaptureComponent2D.TextureTarget` null _returnvalue)
  (bind _output_get (set `self.scene capture 2 d component` _returnvalue))
  (set `self.isBroken?` false)
  (set `SceneCaptureComponent.bCaptureEveryFrame` true _output_get)
  (`KismetSystemLibrary.Delay` 0.2)
  (set `SceneCaptureComponent.bCaptureEveryFrame` false _output_get))

(event `Update camera`
  (set `SceneCaptureComponent2D.TextureTarget` (`self.Texture Target`) (`self.scene capture 2 d component`)))

(event `Break/Fix`
  (`/Engine/EditorBlueprintResources/StandardMacros.FlipFlop`
    (:`A`
      (set `self.isBroken?` true)
      (`NiagaraFunctionLibrary.SpawnSystemAtLocation` "/Game/SecurityCameras/Niagara_Effects/NS_Electricity.NS_Electricity" (`self.K2_GetActorLocation`) (`self.K2_GetActorRotation`) :!label _label)
      (`GameplayStatics.PlaySoundAtLocation` "/Game/SecurityCameras/Sounds/Wav_Electricity.Wav_Electricity" (`self.K2_GetActorLocation`) (struct) 1.0 1.0 0.0 "/Game/SecurityCameras/Sounds/SA_Static_CCTV.SA_Static_CCTV" null null null)
      (`KismetSystemLibrary.Delay` (`KismetMathLibrary.RandomFloatInRange` 4.0 7.0))
      (if (`self.isBroken?`)
        (goto _label)))
    (:`B`
      (`GameplayStatics.PlaySoundAtLocation` "/Game/SecurityCameras/Sounds/Wav_Fix.Wav_Fix" (`self.K2_GetActorLocation`) (struct) 1.0 1.0 0.0 "/Game/SecurityCameras/Sounds/SA_Static_CCTV.SA_Static_CCTV" null null null)
      (`KismetSystemLibrary.Delay` 2.0)
      (set `self.isBroken?` false))))

(fn `UserConstructionScript`)